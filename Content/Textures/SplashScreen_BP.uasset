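; SplashScreen_BP is a splash screen actor that keeps a referenced LayerParent hidden until the player gives input.
; BeginPlay hides the LayerParent root component and its children.
; Pressing Start or B on the joypad, or any non-zero move axis detected on Tick, destroys the splash actor and makes that hierarchy visible again.
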(event EventBeginPlay
  (Rendering|SetVisibility (Variables|/Script/Engine.Actor|GetRootComponent (Variables|Default|GetLayerParent)) false true))

(event Collision|EventActorBeginOverlap
  (params (OtherActor :type Actor%20Object%20Reference)))

(event EventTick
  (params (DeltaSeconds :type Float%20%28single-precision%29))
  (if (or (!= (Input|AxisValues|GetMoveX) 0.0) (!= (Input|AxisValues|GetMoveY) 0.0))
    (Actor|DestroyActor)
    (Rendering|SetVisibility (Variables|/Script/Engine.Actor|GetRootComponent (Variables|Default|GetLayerParent)) true true)))

(event Input|ActionEvents|InputActionJoyPad_B
  (params (Key :type Key%20Structure :default "None"))
  (:Pressed
    (Actor|DestroyActor)
    (Rendering|SetVisibility (Variables|/Script/Engine.Actor|GetRootComponent (Variables|Default|GetLayerParent)) true true)))

(event Input|ActionEvents|InputActionJoyPad_Start
  (params (Key :type Key%20Structure :default "None"))
  (:Pressed
    (Actor|DestroyActor)
    (Rendering|SetVisibility (Variables|/Script/Engine.Actor|GetRootComponent (Variables|Default|GetLayerParent)) true true)))

(fn ConstructionScript)