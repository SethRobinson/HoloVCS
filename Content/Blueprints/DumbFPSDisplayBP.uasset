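; A simple in-world FPS display actor that shows the measured frame rate on a text render component.
; Each Tick increments a frame counter, and once one second of real time has passed it writes the count to the text and resets.
; SetupTimer, also called at BeginPlay, zeroes the counter and sets the next one-second deadline.
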(event EventBeginPlay
  (CallFunction|SetupTimer))

(event EventTick
  (params (DeltaSeconds :type Float%20%28single-precision%29))
  (Variables|Default|SetfpsCounter (+ (Variables|Default|GetfpsCounter) 1))
  (Development|PrintString (Utilities|String|ToString(Float) (Utilities|Time|GetRealTimeSeconds)) false false)
  (if (> (Utilities|Time|GetRealTimeSeconds) (Variables|Default|Gettimer))
    (Rendering|Components|TextRender|SetText (Variables|Default|GetTextRender) (Utilities|Text|ToText(Integer) (Variables|Default|GetfpsCounter)))
    (CallFunction|SetupTimer)))

(fn ConstructionScript)

(fn SetupTimer
  (Variables|Default|SetfpsCounter 0)
  (Variables|Default|Settimer (+ (Utilities|Time|GetRealTimeSeconds) 1.0)))